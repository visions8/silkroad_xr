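; Interactable actor for the VR pawn, with a floating text label and a scale bounce on spawn and touch.
; The construction script sets the label's text and color, and each tick rotates it toward the pawn's camera.
; Sphere overlap with VRPawn_silkroad hides the label and plays the timeline bounce, and leaving shows it again.
; DoOnce gates suppress repeated overlap triggers and bounce restarts.
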(event OnComponentBeginOverlap(SphereCollision)
  (params (OverlappedComponent :type Primitive%20Component%20Object%20Reference) (OtherActor :type Actor%20Object%20Reference) (OtherComp :type Primitive%20Component%20Object%20Reference) (OtherBodyIndex :type Integer) (bFromSweep :type Boolean) (SweepResult :type Hit%20Result%20Structure%20%28by%20ref%29))
  (Utilities|Casting|CastToVRPawn_silkroad OtherActor)
  (Utilities|FlowControl|DoOnce false
    (:Completed
      (Development|PrintString (Utilities|String|Append (Utilities|GetDisplayName OtherComp) " overlapped with " (Utilities|GetDisplayName self)) true true "(R=0.000000,G=0.660000,B=1.000000,A=1.000000)" 5.0)
      (Rendering|SetVisibility (Variables|Default|GetTextRender) false false)
      (Utilities|FlowControl|DoOnce false
        (:Completed
          (CallFunction|BounceActor))))))

(event OnComponentEndOverlap(SphereCollision)
  (params (OverlappedComponent :type Primitive%20Component%20Object%20Reference) (OtherActor :type Actor%20Object%20Reference) (OtherComp :type Primitive%20Component%20Object%20Reference) (OtherBodyIndex :type Integer))
  (Utilities|Casting|CastToVRPawn_silkroad OtherActor)
  (Utilities|FlowControl|Sequence
    (:then_0
      (Utilities|FlowControl|DoOnce false) ; enters at Reset
    )
    (:then_1
      (Rendering|SetVisibility (Variables|Default|GetTextRender) true false))))

(event Custom|BounceActor
  (bind _bounce (Timeline|Timeline PlayFromStart)
    (:Update
      (Transformation|SetActorScale3D (Math|Conversions|ToVector(Float) _bounce)))
    (:Finished
      (Utilities|FlowControl|DoOnce false) ; enters at Reset
    )))

(event EventBeginPlay
  (CallFunction|BounceActor))

(event Collision|EventActorBeginOverlap
  (params (OtherActor :type Actor%20Object%20Reference)))

(event EventTick
  (params (DeltaSeconds :type Float%20%28single-precision%29))
  (CallFunction|RotateTexttoCamera))

(fn ConstructionScript
  (bind _textrender (Variables|Default|GetTextRender))
  (Rendering|Components|TextRender|SetText _textrender (Variables|Default|GetText))
  (Rendering|Components|TextRender|SetTextRenderColor _textrender (Variables|Default|GetTextColor)))

(fn RotateTexttoCamera
  (bind _textrender (Variables|Default|GetTextRender))
  (bind _asvrpawn_silkroad (Utilities|Casting|CastToVRPawn_silkroad (Game|Player|GetPlayerPawn 0)))
  (Transformation|SetWorldRotation _textrender (Math|Rotator|FindLookatRotation (Transformation|GetWorldLocation _textrender) (Transformation|GetWorldLocation (Variables|/Game/CUSTOM/GAME/VRPawn_silkroad.VRPawn_silkroad_C|GetCamera _asvrpawn_silkroad))) false false))