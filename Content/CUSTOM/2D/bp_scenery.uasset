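; Scenery actor that displays layered 2D scene textures on a Plane through a configurable material.
; The construction script creates a dynamic material instance from the Material variable and assigns it to the Plane.
; It then copies the actor's variables into material parameters: surface look, sine strength, two textures, a texture-switch alpha, and opacity and XYZ offsets for three scene layers.
; The event graph holds no runtime logic.
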(event EventBeginPlay)

(event Collision|EventActorBeginOverlap
  (params (OtherActor :type Actor%20Object%20Reference)))

(event EventTick
  (params (DeltaSeconds :type Float%20%28single-precision%29)))

(fn ConstructionScript
  (CallFunction|SetDynamicMaterialInstance))

(fn SetDynamicMaterialInstance
  (bind _returnvalue (Rendering|Material|CreateDynamicMaterialInstance (Variables|Default|GetMaterial) "None" "None" :!class /Script/Engine.KismetMaterialLibrary))
  (Rendering|Material|SetMaterial (Variables|Default|GetPlane) 0 _returnvalue)
  (Utilities|FlowControl|Sequence
    (:then_0
      (Rendering|Material|SetScalarParameterValue _returnvalue "Roughness" (Variables|General|GetRoughness) :!class /Script/Engine.MaterialInstanceDynamic)
      (Rendering|Material|SetScalarParameterValue _returnvalue "TextureScale" (Variables|Default|GetTextureScale) :!class /Script/Engine.MaterialInstanceDynamic)
      (Rendering|Material|SetScalarParameterValue _returnvalue "EmissiveStrength" (Variables|General|GetEmissiveStrength) :!class /Script/Engine.MaterialInstanceDynamic))
    (:then_1
      (Rendering|Material|SetTextureParameterValue _returnvalue "Texture_Scene_0" (Variables|General|GetTexture_0))
      (Rendering|Material|SetTextureParameterValue _returnvalue "Texture_Scene_1" (Variables|General|GetTexture_1)))
    (:then_2
      (Rendering|Material|SetScalarParameterValue _returnvalue "SineStrength" (Variables|Default|GetSineStrength) :!class /Script/Engine.MaterialInstanceDynamic))
    (:then_3
      (Rendering|Material|SetScalarParameterValue _returnvalue "OpacityOffset_Scene_0" (Variables|Opacity|GetOpacityOffset_Scene_0) :!class /Script/Engine.MaterialInstanceDynamic)
      (Rendering|Material|SetScalarParameterValue _returnvalue "OpacityOffset_Scene_1" (Variables|Opacity|GetOpacityOffset_Scene_1) :!class /Script/Engine.MaterialInstanceDynamic)
      (Rendering|Material|SetScalarParameterValue _returnvalue "OpacityOffset_Scene_2" (Variables|Opacity|GetOpacity_Offset_Scene_2) :!class /Script/Engine.MaterialInstanceDynamic)
      (Rendering|Material|SetScalarParameterValue _returnvalue "SwitchTexAlpha" (Variables|Opacity|GetSwitchTexAlpha) :!class /Script/Engine.MaterialInstanceDynamic))
    (:then_4
      (Rendering|Material|SetVectorParameterValue _returnvalue "XYZ_Offset_Scene_0" (Variables|XYZOffset|GetXYZ_Offset_Scene_0) :!class /Script/Engine.MaterialInstanceDynamic)
      (Rendering|Material|SetVectorParameterValue _returnvalue "XYZ_Offset_Scene_1" (Variables|XYZOffset|GetXYZ_Offset_Scene_1) :!class /Script/Engine.MaterialInstanceDynamic)
      (Rendering|Material|SetVectorParameterValue _returnvalue "XYZ_Offset_Scene_2" (Variables|XYZOffset|GetXYZ_Offset_Scene_2) :!class /Script/Engine.MaterialInstanceDynamic))))